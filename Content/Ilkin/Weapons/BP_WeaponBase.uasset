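; Base weapon Blueprint that manages attachment visibility and exposes a shell socket transform.
; AddScopeAttachment and AddFlashlight switch on their input to hide or show the SMT4Sight and TacticalFlashlight components, including their children.
; GetShellTransform returns the world-space transform of the skeletal mesh's ShellSocket.
; BeginPlay, Tick, overlap and the construction script contain no logic.
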(event `/Game/Ilkin/Interfaces/FPS/BI_GunInterface.addScopeAttachment`
  (params (scope :type Integer))
  (bind _sm_t4_sight (`self.SM_T4_Sight`))
  (switch `int` scope
    (:`0`
      (`SceneComponent.SetVisibility` _sm_t4_sight false true))
    (:`1`
      (`SceneComponent.SetVisibility` _sm_t4_sight true true))))

(event `/Game/Ilkin/Interfaces/FPS/BI_GunInterface.addFlashlight`
  (params (flashLight :type Integer))
  (bind _tactical_flashlight (`self.Tactical_flashlight`))
  (switch `int` flashLight
    (:`0`
      (`SceneComponent.SetVisibility` _tactical_flashlight false true))
    (:`1`
      (`SceneComponent.SetVisibility` _tactical_flashlight true true))))

(fn `getShellTransform`
  (returns (transform :type "Transform Structure"))
  (return (`SceneComponent.GetSocketTransform` (`self.SkeletalMesh`) "ShellSocket" "RTS_World")))

(fn `UserConstructionScript`)