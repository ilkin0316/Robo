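; Inventory actor component that lets the player pick up, stack and drop items.
; The pickup input sphere-traces from the follow camera and stores BP_MasterPickUpItem data in a name-keyed map, then destroys the actor.
; Removal respawns items in the world, placing single drops by a downward trace and multi-drops by tracing around the player for a clear side.
; It also spawns BP_recording on BeginPlay and a health pickup when a stack reaches five.
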(event `self.ReceiveBeginPlay`
  (bind _returnvalue (`|SpawnActorFromClass` "/Game/Ilkin/Blueprints/Recording/BP_recording.BP_recording_C" (`KismetMathLibrary.MakeTransform` (10000000.0 0.0 0.0)) "Undefined" "MultiplyWithRoot" null null))
  (set `self.RecordingRef` _returnvalue))

(event `EnhancedInput|/Game/ThirdPerson/Input/Actions/IlkinsInputs/IA_PickUp`
  (params (ActionValue :type Boolean) (ElapsedSeconds :type "Float (double-precision)") (TriggeredSeconds :type "Float (double-precision)") (InputAction :type "InputAction Object Reference" :default "/Game/ThirdPerson/Input/Actions/IlkinsInputs/IA_PickUp.IA_PickUp"))
  (bind _connectedactor (`self.connectedActor`))
  (bind _followcamera (`/Game/ThirdPerson/Blueprints/BP_ThirdPersonCharacter.FollowCamera` _connectedactor))
  (bind _returnvalue (`SceneComponent.K2_GetComponentLocation` _followcamera))
  (:`Completed`
    (bind (_outhit _returnvalue_2) (`KismetSystemLibrary.SphereTraceSingle` :`Start` _returnvalue :`End` (+ _returnvalue (* (`SceneComponent.GetForwardVector` _followcamera) (+ (`SpringArmComponent.TargetArmLength` (`/Game/ThirdPerson/Blueprints/BP_ThirdPersonCharacter.CameraBoom` _connectedactor)) 500.0))) :`Radius` 10.0 :`TraceChannel` "TraceTypeQuery1" :`DrawDebugType` "ForDuration"))
    (if _returnvalue_2
      (bind (_bblockinghit _binitialoverlap _time _distance _location _impactpoint _normal _impactnormal _physmat _hitactor) (`GameplayStatics.BreakHitResult` _outhit))
      (bind _added (`self.TryAddItem` _hitactor))
      (if _added
        (`Actor.K2_DestroyActor` _hitactor)))))

(fn `AddItemtoInventory`
  (params (Item :type "/Game/Ilkin/Blueprints/Structures/S_ItemData Structure"))
  (`BlueprintMapLibrary.Map_Add` (`self.Inventory`) (`.Name_5_B69E13874AF0C487C40D03B56FF35FEC` (break `/Game/Ilkin/Blueprints/Structures/S_ItemData` Item)) Item))

(fn `amount`
  (params (S_ItemData :type "/Game/Ilkin/Blueprints/Structures/S_ItemData Structure (by ref)"))
  (returns (Amount :type Integer))
  (return (`.Amount_17_824E1DA042A1665266DCDCB0C971104C` (break `/Game/Ilkin/Blueprints/Structures/S_ItemData` S_ItemData))))

(fn `getCurrentlyAmount`
  (params (S_ItemData :type "/Game/Ilkin/Blueprints/Structures/S_ItemData Structure (by ref)"))
  (bind _amount (`self.amount` S_ItemData))
  (set `self.currentlyAmount` _amount))

(fn `getStartEndTrace`
  (params (vectorDirection :type "Vector Structure"))
  (returns (Start :type "Vector Structure") (End :type "Vector Structure"))
  (bind _returnvalue (`SceneComponent.K2_GetComponentLocation` (`Character.Mesh` (`self.connectedActor`))))
  (return (+ _returnvalue (0.0 0.0 100.0)) (+ (+ _returnvalue vectorDirection) (0.0 0.0 100.0))))

(fn `IncreaseItemAmount`
  (params (Item :type "/Game/Ilkin/Blueprints/Structures/S_ItemData Structure"))
  (locals (ItemName :type String))
  (bind _value (`BlueprintMapLibrary.Map_Find` (`self.Inventory`) (`local.ItemName`)))
  (bind ((`Amount_17_824E1DA042A1665266DCDCB0C971104C` _amount)) (break `/Game/Ilkin/Blueprints/Structures/S_ItemData` _value))
  (set `local.ItemName` (`.Name_5_B69E13874AF0C487C40D03B56FF35FEC` (break `/Game/Ilkin/Blueprints/Structures/S_ItemData` Item)))
  (bind _result (`/Engine/EditorBlueprintResources/StandardMacros.IncrementInt` _amount)
    (:`  `
      (bind _structout (setmembers `/Game/Ilkin/Blueprints/Structures/S_ItemData` :`StructRef` _value :`Amount` _result))
      (`BlueprintMapLibrary.Map_Add` (`self.Inventory`) (`local.ItemName`) _structout)
      (if (== _amount 5)
        (`KismetSystemLibrary.PrintString` "Hello")
        (`|SpawnActorFromClass` "/Game/Turan/HealthPickUpT/HealthPickUpActor.HealthPickUpActor_C" (`KismetMathLibrary.MakeTransform` (4500.0 1570.0 100.0)) "Undefined" "MultiplyWithRoot" null null)
        (else
          (`KismetSystemLibrary.PrintString` "Bye"))))))

(fn `IsItemAlreadyInventory`
  (params (Item :type "/Game/Ilkin/Blueprints/Structures/S_ItemData Structure"))
  (returns (ReturnValue :type Boolean))
  (return (`BlueprintMapLibrary.Map_Contains` (`self.Inventory`) (`.Name_5_B69E13874AF0C487C40D03B56FF35FEC` (break `/Game/Ilkin/Blueprints/Structures/S_ItemData` Item)))))

(fn `RemoveItemAll`
  (params (ItemName :type String))
  (locals (DeletedItem :type "/Game/Ilkin/Blueprints/Structures/S_ItemData Structure") (DropAmount :type Integer))
  (bind (_value _returnvalue) (`BlueprintMapLibrary.Map_Find` (`self.Inventory`) ItemName))
  (bind (_name _weight _value_2 _description _category _amount) (break `/Game/Ilkin/Blueprints/Structures/S_ItemData` _value))
  (if _returnvalue
    (set `local.DeletedItem` _value)
    (bind _output_get (set `local.DropAmount` _amount))
    (for _ (range 1 (+ _output_get 1))
      (bind _structout (setmembers `/Game/Ilkin/Blueprints/Structures/S_ItemData` :`StructRef` (`local.DeletedItem`) :`Amount` (- _amount 1)))
      (`BlueprintMapLibrary.Map_Add` (`self.Inventory`) (`local.ItemName`) _structout)
      (bind _position (`self.tryTraceAround`))
      (`self.spawnItem` (`.ItemClass_20_0133CC7640DA6362834C26AC7CA1A923` (break `/Game/Ilkin/Blueprints/Structures/S_ItemData` (`local.DeletedItem`))) _position))
    (`BlueprintMapLibrary.Map_Remove` (`self.Inventory`) (`local.ItemName`))
    (return)))

(fn `RemoveItemByAmount`
  (params (item :type String) (amountToDrop :type Integer))
  (returns (updatedItem :type "/Game/Ilkin/Blueprints/Structures/S_ItemData Structure"))
  (locals (foundItem :type "/Game/Ilkin/Blueprints/Structures/S_ItemData Structure"))
  (bind (_value _returnvalue) (`BlueprintMapLibrary.Map_Find` (`self.Inventory`) item))
  (bind _value_2 (`BlueprintMapLibrary.Map_Find` (`self.Inventory`) (`local.item`)))
  (if _returnvalue
    (set `local.foundItem` _value)
    (for _ (range amountToDrop)
      (bind _structout (setmembers `/Game/Ilkin/Blueprints/Structures/S_ItemData` :`StructRef` (`local.foundItem`) :`Amount` (- (`.Amount_17_824E1DA042A1665266DCDCB0C971104C` (break `/Game/Ilkin/Blueprints/Structures/S_ItemData` _value)) 1)))
      (`BlueprintMapLibrary.Map_Add` (`self.Inventory`) (`local.item`) _structout)
      (bind _position (`self.tryTraceAround`))
      (`self.spawnItem` (`.ItemClass_20_0133CC7640DA6362834C26AC7CA1A923` (break `/Game/Ilkin/Blueprints/Structures/S_ItemData` (`local.foundItem`))) _position))
    (if (== (`.Amount_17_824E1DA042A1665266DCDCB0C971104C` (break `/Game/Ilkin/Blueprints/Structures/S_ItemData` _value_2)) 0)
      (`BlueprintMapLibrary.Map_Remove` (`self.Inventory`) (`local.item`))
      (return)
      (else
        (return _value_2)))))

(fn `RemoveSingleItem`
  (params (Key :type "String (by ref)"))
  (returns (itemFullRemoved :type Boolean) (newItemData :type "/Game/Ilkin/Blueprints/Structures/S_ItemData Structure"))
  (locals (DeletedItem :type "/Game/Ilkin/Blueprints/Structures/S_ItemData Structure"))
  (bind (_value _returnvalue) (`BlueprintMapLibrary.Map_Find` (`self.Inventory`) Key))
  (bind (_name _weight _value_2 _description _category _amount) (break `/Game/Ilkin/Blueprints/Structures/S_ItemData` _value))
  (if _returnvalue
    (if (> _amount 1)
      (bind _structout (setmembers `/Game/Ilkin/Blueprints/Structures/S_ItemData` :`StructRef` _value :`Amount` (- _amount 1)))
      (`BlueprintMapLibrary.Map_Add` (`self.Inventory`) (`local.Key`) _structout)
      (bind _impactpoint (`self.traceFromAbove`))
      (`self.spawnItem` (`.ItemClass_20_0133CC7640DA6362834C26AC7CA1A923` (break `/Game/Ilkin/Blueprints/Structures/S_ItemData` _structout)) _impactpoint)
      (return false _structout)
      (else
        (bind _output_get (set `local.DeletedItem` _value))
        (`BlueprintMapLibrary.Map_Remove` (`self.Inventory`) (`local.Key`))
        (bind _impactpoint_2 (`self.traceFromAbove`))
        (`self.spawnItem` (`.ItemClass_20_0133CC7640DA6362834C26AC7CA1A923` (break `/Game/Ilkin/Blueprints/Structures/S_ItemData` _output_get)) _impactpoint_2)
        (return true)))))

(fn `spawnItem`
  (params (Class :type "Actor Class Reference") (Position :type "Vector Structure"))
  (`|SpawnActorFromClass` Class (`KismetMathLibrary.MakeTransform` (+ Position (0.0 0.0 50.0))) "Undefined" "MultiplyWithRoot" null null))

(fn `traceFromAbove`
  (returns (ImpactPoint :type "Vector Structure"))
  (bind _connectedactor (`self.connectedActor`))
  (bind _returnvalue (`SceneComponent.K2_GetComponentLocation` (`Character.Mesh` _connectedactor)))
  (bind _x (.x (* (`SceneComponent.GetForwardVector` (`/Game/ThirdPerson/Blueprints/BP_ThirdPersonCharacter.FollowCamera` _connectedactor)) 200.0)))
  (bind _y (.y (* (`SceneComponent.GetForwardVector` (`/Game/ThirdPerson/Blueprints/BP_ThirdPersonCharacter.FollowCamera` _connectedactor)) 200.0)))
  (bind (_outhit _returnvalue_2) (`KismetSystemLibrary.SphereTraceSingle` (+ _returnvalue (`KismetMathLibrary.MakeVector` _x _y 2000.0)) (+ _returnvalue (`KismetMathLibrary.MakeVector` _x _y -100.0)) 5.0 "TraceTypeQuery1"))
  (if _returnvalue_2
    (bind (_bblockinghit _binitialoverlap _time _distance _location _impactpoint _normal _impactnormal _physmat _hitactor _hitcomponent _hitbonename _bonename _hititem _elementindex _faceindex _tracestart _traceend) (`GameplayStatics.BreakHitResult` _outhit))
    (return _impactpoint)
    (else
      (return _traceend))))

(fn `TryAddItem`
  (params (HitActor :type "Actor Object Reference"))
  (returns (added :type Boolean))
  (locals (CurrentItem :type "/Game/Ilkin/Blueprints/Structures/S_ItemData Structure"))
  (bind _currentitem (`local.CurrentItem`))
  (bind _asbp_master_pick_up_item (cast `/Game/Ilkin/Blueprints/Items/BP_MasterPickUpItem` HitActor)
    (:`then`
      (bind _output_get (set `local.CurrentItem` (`/Game/Ilkin/Blueprints/Items/BP_MasterPickUpItem.GetItemData` _asbp_master_pick_up_item)))
      (if (`self.IsItemAlreadyInventory` _output_get)
        (`self.IncreaseItemAmount` _currentitem)
        (else
          (`self.AddItemtoInventory` _currentitem)))
      (`KismetSystemLibrary.PrintString` (`KismetStringLibrary.Concat_StrStr` (`.Name_5_B69E13874AF0C487C40D03B56FF35FEC` (break `/Game/Ilkin/Blueprints/Structures/S_ItemData` _currentitem)) "Added"))
      (return true))
    (:`CastFailed`
      (set `local.CurrentItem` (struct))
      (return false))))

(fn `tryTraceAround`
  (returns (position :type "Vector Structure"))
  (bind (_start _end) (`self.getStartEndTrace` (* (`Actor.GetActorForwardVector` (`self.connectedActor`)) 100.0)))
  (bind (_outhit _returnvalue) (`KismetSystemLibrary.SphereTraceSingle` _start _end 10.0 "TraceTypeQuery1"))
  (if _returnvalue
    (bind (_start_2 _end_2) (`self.getStartEndTrace` (* (`Actor.GetActorRightVector` (`self.connectedActor`)) 100.0)))
    (bind (_outhit_2 _returnvalue_2) (`KismetSystemLibrary.SphereTraceSingle` _start_2 _end_2 10.0 "TraceTypeQuery1"))
    (if _returnvalue_2
      (bind (_start_3 _end_3) (`self.getStartEndTrace` (* (`Actor.GetActorForwardVector` (`self.connectedActor`)) -100.0)))
      (bind (_outhit_3 _returnvalue_3) (`KismetSystemLibrary.SphereTraceSingle` _start_3 _end_3 10.0 "TraceTypeQuery1"))
      (if _returnvalue_3
        (bind (_start_4 _end_4) (`self.getStartEndTrace` (* (`Actor.GetActorRightVector` (`self.connectedActor`)) -100.0)))
        (bind (_outhit_4 _returnvalue_4) (`KismetSystemLibrary.SphereTraceSingle` _start_4 _end_4 10.0 "TraceTypeQuery1"))
        (if _returnvalue_4
          (bind (_bblockinghit _binitialoverlap _time _distance _location _impactpoint _normal _impactnormal _physmat _hitactor _hitcomponent _hitbonename _bonename _hititem _elementindex _faceindex _tracestart _traceend) (`GameplayStatics.BreakHitResult` _outhit_4))
          (return _impactpoint)
          (else
            (return _traceend)))
        (else
          (return (`.TraceEnd` (`GameplayStatics.BreakHitResult` _outhit_3)))))
      (else
        (return (`.TraceEnd` (`GameplayStatics.BreakHitResult` _outhit_2)))))
    (else
      (return (`.TraceEnd` (`GameplayStatics.BreakHitResult` _outhit))))))