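; Preview actor that shows a swappable static mesh to a SceneCaptureComponent2D, with drag-to-rotate and zoom controls.
; UpdateStaticMesh applies a supplied mesh, camera position and zoom limits, while ResetMesh clears the mesh.
; Click events gate rotation, and MoveMouse turns scaled mouse deltas into world pitch and yaw on the mesh.
; Zoom offsets the capture component only while its resulting relative X stays within the stored limits.
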(event `ClickedStart`
  (params (MouseClickedPosition :type "Vector2D Structure"))
  (set `self.MouseClickedPosition` MouseClickedPosition)
  (set `self.canRotate` true))

(event `ClickedEnd`
  (set `self.canRotate` false))

(event `MoveMouse`
  (params (MouseLocation :type "Vector2D Structure"))
  (bind (_x _y) (`KismetMathLibrary.BreakVector2D` (/ (- MouseLocation (`self.MouseClickedPosition`)) (4.0 4.0))))
  (if (`self.canRotate`)
    (`SceneComponent.K2_AddWorldRotation` (`self.StaticMesh`) (`KismetMathLibrary.MakeRotator` 0.0 _y (* _x -1.0)) false false)
    (set `self.MouseClickedPosition` MouseLocation)))

(event `Zoom`
  (params (ZoomAmount :type "Vector Structure"))
  (bind _scenecapturecomponent2d (`self.SceneCaptureComponent2D`))
  (bind _returnvalue (+ (`SceneComponent.RelativeLocation` _scenecapturecomponent2d) ZoomAmount))
  (bind _x (.x _returnvalue))
  (if (and (< _x (`self.MinPosition`)) (> _x (`self.MaxPosition`)))
    (`SceneComponent.K2_SetRelativeLocation` _scenecapturecomponent2d _returnvalue false false)))

(fn `ResetMesh`
  (`StaticMeshComponent.SetStaticMesh` (`self.StaticMesh`) null))

(fn `UpdatePosition`
  (params (MinPosition :type "Float (double-precision)") (MaxPosition :type "Float (double-precision)"))
  (set `self.MinPosition` MinPosition)
  (set `self.MaxPosition` MaxPosition))

(fn `UpdateStaticMesh`
  (params (NewParam :type "/Game/Ilkin/Blueprints/Recording/S_RecordingSettings Structure"))
  (bind (_mesh _cameraposition _maxposition _minposition) (break `/Game/Ilkin/Blueprints/Recording/S_RecordingSettings` NewParam))
  (if (!= _mesh null)
    (`StaticMeshComponent.SetStaticMesh` (`self.StaticMesh`) _mesh)
    (`SceneComponent.K2_SetRelativeLocation` (`self.SceneCaptureComponent2D`) _cameraposition false false)
    (`self.UpdatePosition` _minposition _maxposition)))

(fn `UserConstructionScript`)