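; BP_TrshCan is a trash can actor that acts as the win trigger for dropping off pickup items.
; Each BP_MasterPickUpItem that begins overlapping its Box increments CurrentlyAmount on ACInventory, without destroying the item.
; When the count equals two, it shows the WB_Win widget and pauses the game after a short delay; other counts only print a debug string.
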(event `self.Box.OnComponentBeginOverlap`
  (params (OverlappedComponent :type "PrimitiveComponent Object Reference") (OtherActor :type "Actor Object Reference") (OtherComp :type "PrimitiveComponent Object Reference") (OtherBodyIndex :type Integer) (bFromSweep :type Boolean) (SweepResult :type "HitResult Structure (by ref)"))
  (bind _ac_inventory (`self.AC_Inventory`))
  (cast `/Game/Ilkin/Blueprints/Items/BP_MasterPickUpItem` OtherActor)
  (bind _output_get (set `/Game/Ilkin/Blueprints/ActorComponents/AC_Inventory.currentlyAmount` (+ (`/Game/Ilkin/Blueprints/ActorComponents/AC_Inventory.currentlyAmount` _ac_inventory) 1) _ac_inventory))
  (if (== _output_get 2)
    (bind _returnvalue (`|CreateWidget` "/Game/Ilkin/Widgets/WB_Win.WB_Win_C"))
    (`UserWidget.AddToViewport` _returnvalue 0)
    (`KismetSystemLibrary.Delay` 1.0)
    (`GameplayStatics.SetGamePaused` true)
    (else
      (`KismetSystemLibrary.PrintString` "Olmadi"))))

(fn `UserConstructionScript`)