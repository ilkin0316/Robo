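; BP_MasterPickUpItem is, by its name, the master Blueprint for pickup items, holding the data that describes an item.
; GetItemData packs its item variables, including name, category, amount, class and recording settings, into an SItemData struct.
; GetCurrentAmount reads the amount from a given SItemData through the Amounttt helper, stores it in CurrentAmount and returns it.
; The event graph and construction script are empty, so no pickup logic appears here.
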(fn `amounttt`
  (params (S_ItemData :type "/Game/Ilkin/Blueprints/Structures/S_ItemData Structure (by ref)"))
  (returns (Amount :type Integer))
  (return (`.Amount_17_824E1DA042A1665266DCDCB0C971104C` (break `/Game/Ilkin/Blueprints/Structures/S_ItemData` S_ItemData))))

(fn `getCurrentAmount`
  (params (S_ItemData :type "/Game/Ilkin/Blueprints/Structures/S_ItemData Structure (by ref)"))
  (returns (Output_Get :type Integer))
  (bind _amount (`self.amounttt` S_ItemData))
  (bind _output_get (set `self.currentAmount` _amount))
  (return _output_get))

(fn `GetItemData`
  (returns (NewParam :type "/Game/Ilkin/Blueprints/Structures/S_ItemData Structure"))
  (return (make `/Game/Ilkin/Blueprints/Structures/S_ItemData` (`self.Name`) (`self.Weight`) (`self.Value`) (`self.Description`) (`self.Category`) (`self.Amount`) (`self.itemClass`) (`self.Recorgind Settings`))))

(fn `UserConstructionScript`)